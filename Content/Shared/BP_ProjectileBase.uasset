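; Base projectile Blueprint that handles spawn, flight and impact audio and VFX, with each asset played only if it is valid.
; On BeginPlay it plays a spawn sound, attaches a flight sound that stops when the projectile is destroyed, and spawns VFX facing its forward vector.
; The OnSpawnProjectileHitFX event plays the impact sound and spawns impact VFX at the supplied hit location.
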(event `self.ReceiveBeginPlay`
  (`|ExecutionSequence`
    (:`then_0`
      (bind _spawnsound (`self.SpawnSound`)
        (:`then`
          (`GameplayStatics.PlaySoundAtLocation` _spawnsound (`self.K2_GetActorLocation`) (struct) 1.0 1.0 0.0 null null null null))
        (:`else`)))
    (:`then_1`
      (bind _flyinsound (`self.FlyinSound`)
        (:`then`
          (`GameplayStatics.SpawnSoundAttached` _flyinsound (`self.RootComponent`) "None" (0.0 0.0 0.0) (struct) "KeepRelativeOffset" true 1.0 1.0 0.0 null null))
        (:`else`)))
    (:`then_2`
      (bind _spawnvfx (`self.SpawnVFX`)
        (:`then`
          (`NiagaraFunctionLibrary.SpawnSystemAtLocation` _spawnvfx (`self.K2_GetActorLocation`) (`KismetMathLibrary.Conv_VectorToRotator` (`self.GetActorForwardVector`))))
        (:`else`)))))

(event `self.BP_OnSpawnProjectileHitFX`
  (params (HitLocation :type "Vector Structure (by ref)"))
  (`|ExecutionSequence`
    (:`then_0`
      (bind _impactsound (`self.ImpactSound`)
        (:`then`
          (`GameplayStatics.PlaySoundAtLocation` _impactsound HitLocation (struct) 1.0 1.0 0.0 null null null null))
        (:`else`)))
    (:`then_1`
      (bind _impactvfx (`self.ImpactVFX`)
        (:`then`
          (`NiagaraFunctionLibrary.SpawnSystemAtLocation` _impactvfx HitLocation))
        (:`else`)))))

(fn `UserConstructionScript`)